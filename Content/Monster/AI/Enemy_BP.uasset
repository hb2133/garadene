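; Melee enemy character Blueprint that chases the player's ThirdPersonCharacter, attacks it and dies when its health runs out.
; BeginPlay finds the player after a delay, starts a repeating AI MoveTo loop, sets controller focus and attaches a spawned weapon to the sword socket.
; AttackRange overlap loops an attack montage, while sword overlap deals damage gated by CanHitR.
; Death stops movement and destroys enemy and weapon after a random delay; StartRagdoll enables physics separately.
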(event OnComponentBeginOverlap(AttackRange)
  (params (OverlappedComponent :type Primitive%20Component%20Object%20Reference) (OtherActor :type Actor%20Object%20Reference) (OtherComp :type Primitive%20Component%20Object%20Reference) (OtherBodyIndex :type Integer) (bFromSweep :type Boolean) (SweepResult :type Hit%20Result%20Structure%20%28by%20ref%29))
  (if (and (== OtherActor (Variables|Default|GetMy%20Enemy)) (not (Variables|Default|GetIsAttacking)))
    (Variables|Default|SetCanAttack true)
    (Variables|Default|SetIsAttacking true :!label _label)
    (Animation|Montage|PlayMontage (Variables|Character|GetMesh) "/Game/Monster/AI/Corpse_Alert_Attack_Fast2_Montage.Corpse_Alert_Attack_Fast2_Montage"
      (:OnCompleted
        (Variables|Default|SetIsAttacking false)
        (if (and (Variables|Default|GetCanAttack) (Variables|Default|GetIsAlive))
          (goto _label))))))

(event OnComponentEndOverlap(AttackRange)
  (params (OverlappedComponent :type Primitive%20Component%20Object%20Reference) (OtherActor :type Actor%20Object%20Reference) (OtherComp :type Primitive%20Component%20Object%20Reference) (OtherBodyIndex :type Integer))
  (if (and (== OtherActor (Variables|Default|GetMy%20Enemy)) (Variables|Default|GetCanAttack))
    (Variables|Default|SetCanAttack false)))

(event OnComponentBeginOverlap(SwordCollision_R)
  (params (OverlappedComponent :type Primitive%20Component%20Object%20Reference) (OtherActor :type Actor%20Object%20Reference) (OtherComp :type Primitive%20Component%20Object%20Reference) (OtherBodyIndex :type Integer) (bFromSweep :type Boolean) (SweepResult :type Hit%20Result%20Structure%20%28by%20ref%29))
  (if (and (== OtherActor (Variables|Default|GetMy%20Enemy)) (Variables|Default|GetCanHit_R))
    (Variables|Default|SetCanHit_R false)
    (Default|TakeDamage (Variables|Default|GetMy%20Enemy) 35.0)))

(event Custom|GetEnemy
  ;[1 1 1] AI
  (Utilities|FlowControl|Delay 1.0)
  (bind _outactors (Actor|GetAllActorsOfClass "/Game/ThirdPersonCPP/Blueprints/ThirdPersonCharacter.ThirdPersonCharacter_C"))
  (Variables|Default|SetMy%20Enemy (Utilities|Array|Get(acopy) _outactors)))

(event Custom|BaseMovement
  ;[1 1 1] AI
  (Utilities|IsValid (Variables|Default|GetMy%20Enemy) :!label _label
    (:Is%20Valid
      (if (Variables|Default|GetIsAlive)
        (AI|AIMoveTo self "0, 0, 0" (Variables|Default|GetMy%20Enemy) 75.0 false
          (:OnSuccess
            ;;[1 1 1] 공격후 정지시간
            (Utilities|FlowControl|Delay 3.0)
            (goto _label))
          (:OnFail
            (goto _label)))))
    (:Is%20Not%20Valid
      ;;[1 1 1] Nav시작시간
      (Utilities|FlowControl|Delay 1.0)
      (goto _label))))

(event Custom|TakeDamage
  (params (Amount :type Float%20%28single-precision%29))
  (bind _output_get (Variables|Default|SetHealth (- (Variables|Default|GetHealth) Amount)))
  (if (> _output_get 0.0)
    (Development|PrintString (Utilities|String|ToString(Float) (Variables|Default|GetHealth)) true true "(R=1.000000,G=0.000000,B=0.026892,A=1.000000)")
    (else
      (CallFunction|Die))))

(event Custom|Die
  (Variables|Default|SetIsAlive false)
  (Components|Movement|StopMovementImmediately (Variables|Character|GetCharacterMovement))
  (AI|ClearFocus (Variables|Default|GetAIController))
  (Utilities|FlowControl|Delay (Math|Conversions|ToFloat(Integer) (Math|Random|RandomIntegerinRange 4 6)))
  (Actor|DestroyActor)
  (Actor|DestroyActor (Variables|Default|GetEnemy_Weapon)))

(event Custom|StartRagdoll
  (bind _mesh (Variables|Character|GetMesh))
  (Class|SkeletalMeshComponent|SetAllBodiesSimulatePhysics _mesh true)
  (Collision|SetCollisionProfileName _mesh "Ragdoll" true :!class /Script/Engine.PrimitiveComponent)
  (Collision|SetCollisionEnabled (Variables|Collision|GetCapsuleComponent) "NoCollision"))

(event EventBeginPlay
  (Utilities|FlowControl|Sequence
    (:then_0
      ;[1 1 1] AI
      (CallFunction|GetEnemy))
    (:then_1
      (CallFunction|BaseMovement))
    (:then_2
      (bind _asai_controller_enemy_bp (Utilities|Casting|CastToAI_Controller_Enemy_BP (Pawn|GetController)))
      (Variables|Default|SetAIController _asai_controller_enemy_bp)
      (AI|SetFocus (Variables|Default|GetAIController) (Variables|Default|GetMy%20Enemy)))
    (:then_3
      ;[1 1 1] 무기 액터 장착
      (bind _returnvalue (Game|SpawnActorfromClass "/Game/Monster/AI/Enemy_Weapon.Enemy_Weapon_C" (Math|Transform|MakeTransform "0, 0, 0") "Undefined" 0 0))
      (bind _output_get (Variables|Default|SetEnemy_Weapon _returnvalue))
      (Transformation|AttachComponentToComponent _output_get (Variables|Character|GetMesh) "SwordSocket" "SnapToTarget" "SnapToTarget" "SnapToTarget" true))))

(fn ConstructionScript)